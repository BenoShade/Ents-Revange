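; Bullet actor that homes in on an assigned enemy and damages enemy AI it overlaps.
; Tick moves it at Speed toward EnemToAttack, storing the offset to that target in LastLocation, which it later treats as a world position to steer toward if the target becomes invalid.
; Mesh overlap subtracts Damage from an EnemyAi's Health and destroys that enemy at zero or below, leaving the bullet alive.
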(event `self.ReceiveTick`
  (params (DeltaSeconds :type "Float (single-precision)"))
  (bind _enem_to_attack (`self.Enem To attack`))
  (bind _returnvalue (- (`self.K2_GetActorLocation` _enem_to_attack) (`self.K2_GetActorLocation`)))
  (`/Engine/EditorBlueprintResources/StandardMacros.IsValid` _enem_to_attack
    (:`Is Valid`
      (`self.K2_AddActorWorldOffset` (* (`KismetMathLibrary.Normal` _returnvalue) (* DeltaSeconds (`self.Speed`))))
      (`/Engine/EditorBlueprintResources/StandardMacros.IsValid` _enem_to_attack
        (:`Is Valid`
          (set `self.last location` _returnvalue))))
    (:`Is Not Valid`
      (`self.K2_AddActorWorldOffset` (* (`KismetMathLibrary.Normal` (- (`self.last location`) (`self.K2_GetActorLocation`)) 0.0) (* (`self.Speed`) DeltaSeconds))))))

(event `self.StaticMesh.OnComponentBeginOverlap`
  (params (OverlappedComponent :type "PrimitiveComponent Object Reference") (OtherActor :type "Actor Object Reference") (OtherComp :type "PrimitiveComponent Object Reference") (OtherBodyIndex :type Integer) (bFromSweep :type Boolean) (SweepResult :type "HitResult Structure (by ref)"))
  (`|ExecutionSequence`
    (:`then_0`
      (bind _asenemy_ai (cast `/Game/Blueprint/EnemyAi` OtherActor))
      (bind _output_get (set `/Game/Blueprint/EnemyAi.Health` (- (`/Game/Blueprint/EnemyAi.Health` _asenemy_ai) (`self.damage`)) _asenemy_ai))
      (if (<= _output_get 0.0)
        (`self.K2_DestroyActor` _asenemy_ai)))))

(fn `UserConstructionScript`)
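; Test tower actor that automatically shoots bullets at EnemyAi actors within range of its collision sphere.
; Sphere overlaps add and remove enemies from a list; the first entry starts a looping attack timer through a DoOnce, and an empty list clears and resets it.
; Each tick of the timer spawns a Bullet at the shooting point and assigns the first listed enemy as its target.
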(event `self.Sphere collision.OnComponentBeginOverlap`
  (params (OverlappedComponent :type "PrimitiveComponent Object Reference") (OtherActor :type "Actor Object Reference") (OtherComp :type "PrimitiveComponent Object Reference") (OtherBodyIndex :type Integer) (bFromSweep :type Boolean) (SweepResult :type "HitResult Structure (by ref)"))
  (bind _asenemy_ai (cast `/Game/Blueprint/EnemyAi` OtherActor))
  (`KismetArrayLibrary.Array_Add` (`self.List of enemyAI`) _asenemy_ai)
  (`/Engine/EditorBlueprintResources/StandardMacros.DoOnce` false :!label _label
    (:`Completed`
      (`KismetSystemLibrary.K2_SetTimer` null "AttackEnemyAi" 0.8 true))))

(event `self.Sphere collision.OnComponentEndOverlap`
  (params (OverlappedComponent :type "PrimitiveComponent Object Reference") (OtherActor :type "Actor Object Reference") (OtherComp :type "PrimitiveComponent Object Reference") (OtherBodyIndex :type Integer))
  (bind _asenemy_ai (cast `/Game/Blueprint/EnemyAi` OtherActor))
  (`KismetArrayLibrary.Array_RemoveItem` (`self.List of enemyAI`) _asenemy_ai)
  (if (== (`KismetArrayLibrary.Array_Length` (`self.List of enemyAI`)) 0)
    (`KismetSystemLibrary.K2_ClearTimer` null "AttackEnemyAi")
    (goto _label :!via `Reset`)))

(fn `AttackEnemyAI`
  (bind _list_of_enemyai (`self.List of enemyAI`))
  (if (!= (`KismetArrayLibrary.Array_Length` _list_of_enemyai) 0)
    (bind _returnvalue (`|SpawnActorFromClass` "/Game/Blueprint/Bullet.Bullet_C" (`SceneComponent.K2_GetComponentToWorld` (`self.Shooting point`)) "Undefined" "OverrideRootScale" null null))
    (`KismetSystemLibrary.PrintString` "Hello")
    (set `/Game/Blueprint/Bullet.Enem To attack` (`|GetArrayItem` _list_of_enemyai) _returnvalue)))

(fn `UserConstructionScript`)
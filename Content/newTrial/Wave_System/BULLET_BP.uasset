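; Homing bullet actor for the wave system that damages enemies and destroys itself after a short lifetime.
; Each Tick it moves unswept toward EnemyToAttack, or toward that target's last known location once it becomes invalid.
; Mesh overlap uses a cast chain over four enemy classes to subtract Damage from class-specific health variables.
; A lethal hit triggers loot, except for FinalBoss, then destroys enemy and bullet; non-lethal hits leave the bullet alive.
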(event `self.ReceiveBeginPlay`
  (`KismetSystemLibrary.PrintString` (`KismetStringLibrary.Conv_DoubleToString` (`self.Damage`)))
  (`KismetSystemLibrary.Delay` 1.3)
  (`self.K2_DestroyActor`))

(event `self.ReceiveTick`
  (params (DeltaSeconds :type "Float (single-precision)"))
  (bind _enemy_to_attack (`self.Enemy to attack`))
  (bind _returnvalue (`self.K2_GetActorLocation` _enemy_to_attack))
  (`/Engine/EditorBlueprintResources/StandardMacros.IsValid` _enemy_to_attack
    (:`Is Valid`
      (`self.K2_AddActorWorldOffset` (* (`KismetMathLibrary.Normal` (- _returnvalue (`self.K2_GetActorLocation`)) 0.0) (* DeltaSeconds (`self.Speed`))))
      (`/Engine/EditorBlueprintResources/StandardMacros.IsValid` _enemy_to_attack
        (:`Is Valid`
          (set `self.Last Location` _returnvalue))))
    (:`Is Not Valid`
      (`self.K2_AddActorWorldOffset` (* (`KismetMathLibrary.Normal` (- (`self.Last Location`) (`self.K2_GetActorLocation`)) 0.0) (* (`self.Speed`) DeltaSeconds))))))

(event `self.StaticMesh.OnComponentBeginOverlap`
  (params (OverlappedComponent :type "PrimitiveComponent Object Reference") (OtherActor :type "Actor Object Reference") (OtherComp :type "PrimitiveComponent Object Reference") (OtherBodyIndex :type Integer) (bFromSweep :type Boolean) (SweepResult :type "HitResult Structure (by ref)"))
  (bind _astesttt (cast `/Game/newTrial/Wave_System/TESTTT` OtherActor)
    (:`then`
      (`KismetSystemLibrary.PrintString` (`KismetStringLibrary.Conv_DoubleToString` (`self.Damage`)))
      (bind _output_get (set `/Game/newTrial/Wave_System/TESTTT.Health` (- (`/Game/newTrial/Wave_System/TESTTT.Health` _astesttt) (`self.Damage`)) _astesttt))
      (if (<= _output_get 0.0)
        (`/Game/newTrial/Wave_System/TESTTT.Loot2` _astesttt)
        (`self.K2_DestroyActor` _astesttt :!label _label)
        (`self.K2_DestroyActor` (stale _astesst_2))
        (`self.K2_DestroyActor` (stale _asboss))
        (`self.K2_DestroyActor` (stale _asfinal_boss))
        (`self.K2_DestroyActor`)))
    (:`CastFailed`
      (bind _astesst_2 (cast `/Game/newTrial/Wave_System/Tesst2` OtherActor)
        (:`then`
          (bind _output_get_2 (set `/Game/newTrial/Wave_System/Tesst2.Health2` (- (`/Game/newTrial/Wave_System/Tesst2.Health2` _astesst_2) (`self.Damage`)) _astesst_2))
          (if (<= _output_get_2 0.0)
            (`/Game/newTrial/Wave_System/Tesst2.Loot` _astesst_2)
            (goto _label)))
        (:`CastFailed`
          (bind _asboss (cast `/Game/newTrial/Wave_System/BOSS` OtherActor)
            (:`then`
              (bind _output_get_3 (set `/Game/newTrial/Wave_System/BOSS.Health_BOSS` (- (`/Game/newTrial/Wave_System/BOSS.Health_BOSS` _asboss) (`self.Damage`)) _asboss))
              (if (<= _output_get_3 0.0)
                (`/Game/newTrial/Wave_System/BOSS.Loot3` _asboss)
                (goto _label)))
            (:`CastFailed`
              (bind _asfinal_boss (cast `/Game/newTrial/Wave_System/FinalBoss` OtherActor))
              (bind _output_get_4 (set `/Game/newTrial/Wave_System/FinalBoss.Health_finalBOSS` (- (`/Game/newTrial/Wave_System/FinalBoss.Health_finalBOSS` _asfinal_boss) (`self.Damage`)) _asfinal_boss))
              (if (<= _output_get_4 0.0)
                (goto _label)))))))))

(fn `UserConstructionScript`)
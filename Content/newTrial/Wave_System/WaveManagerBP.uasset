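; Wave manager Blueprint that runs enemy waves on a countdown, with an event to skip the wait.
; On BeginPlay it sorts all WaveSpawnPointBP actors into six arrays by spawner type.
; Each wave reads its data table row by wave number and spawns enemies at random matching points through a macro with delays.
; It polls until all tracked enemies are invalid, then advances the wave and restarts the countdown, calling OpenLevel at wave 19.
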(event `self.ReceiveBeginPlay`
  ;[1 1 1] Spawner References and division of each individual array
  (bind _outactors (`GameplayStatics.GetAllActorsOfClass` "/Game/newTrial/Wave_System/WaveSpawnPointBP.WaveSpawnPointBP_C"))
  (bind _output_get (set `self.EnemySpawnPoints` _outactors))
  (for _array_element _output_get
    (switch `/Game/newTrial/Wave_System/Enemy_Type_E` (`/Game/newTrial/Wave_System/WaveSpawnPointBP.SpawnerType` _array_element)
      (:`NewEnumerator0`
        (`KismetArrayLibrary.Array_Add` (`self.E_Ground`) _array_element))
      (:`NewEnumerator1`
        (`KismetArrayLibrary.Array_Add` (`self.E_Air`) _array_element))
      (:`NewEnumerator2`
        (`KismetArrayLibrary.Array_Add` (`self.E_Special`) _array_element))
      (:`NewEnumerator3`
        (`KismetArrayLibrary.Array_Add` (`self.Ground2`) _array_element))
      (:`NewEnumerator4`
        (`KismetArrayLibrary.Array_Add` (`self.Air2`) _array_element))
      (:`NewEnumerator5`
        (`KismetArrayLibrary.Array_Add` (`self.Special2`) _array_element))))
  (`KismetSystemLibrary.Delay` 5.0)
  (`self.Start Countdown`))

(event `Start Countdown`
  ;[1 1 1] timer
  (bind _returnvalue (`KismetSystemLibrary.K2_SetTimerDelegate` (delegate `Count`) 1.0 true))
  (set `self.Time` 40))

(event `Count`
  ;[1 1 1] timer
  (`KismetSystemLibrary.PrintString` (`KismetStringLibrary.Conv_IntToString` (`self.Time`)))
  (if (== (`self.Time`) 0)
    (`KismetSystemLibrary.K2_ClearAndInvalidateTimerHandle` (stale `Start Countdown` _returnvalue) :!label _label)
    (`self.Begine Wave`)
    (else
      (`/Engine/EditorBlueprintResources/StandardMacros.DecrementInt` (`self.Time`)))))

(event `CustomEvent_1`
  ;[1 1 1] timer
  (set `self.Time` 0)
  (goto _label))

(event `Begine Wave`
  ;[1 1 1] Sapwn enemy
  (bind _returnvalue (`|GetDataTableRow` (`self.Enemy data Table`) (`KismetStringLibrary.Conv_StringToName` (`KismetStringLibrary.Conv_IntToString` (`self.WaveNumber`))))
    (:`then`
      (for _array_element (`.EnemiesInfos_4_05D9B68948CCC0F0C05A4CA0FE562DF8` (break `/Game/newTrial/Wave_System/Wave_Info` _returnvalue))
        (`self.NewMacro_1` _array_element))
      (`self.Start Checking if enemies are dead`))
    (:`RowNotFound`
      (`KismetSystemLibrary.PrintString` "no raw"))))

(event `Start Checking if enemies are dead`
  (bind _are_dead_1 (`self.CheckIfAllEnemiesAreDead` :!label _label_2))
  (if _are_dead_1
    (`/Engine/EditorBlueprintResources/StandardMacros.IncrementInt` (`self.WaveNumber`)
      (:`  `
        (if (== (`self.WaveNumber`) 19)
          (`GameplayStatics.OpenLevel` "None"))
        (`KismetSystemLibrary.Delay` 10.0)
        (`self.Start Countdown`)))
    (else
      (`KismetSystemLibrary.Delay` 2.0)
      (goto _label_2))))

(fn `CheckIfAllEnemiesAreDead`
  (returns (`Are Dead?1` :type Boolean))
  (locals (`Are Dead?` :type Boolean :default false))
  (set `local.Are Dead?` true)
  (for _array_element (`self.current enemies`)
    (`/Engine/EditorBlueprintResources/StandardMacros.IsValid` _array_element
      (:`Is Valid`
        (set `local.Are Dead?` false))))
  (return (`local.Are Dead?`)))

(fn `Spawn Enemies`
  (params (Enemy_Info :type "/Game/newTrial/Wave_System/Enemy_Info Structure (by ref)"))
  (locals (EnemyInfoRef :type "/Game/newTrial/Wave_System/Enemy_Info Structure")))

(fn `UserConstructionScript`)
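; Seed spawner Blueprint that opens a seed selection menu when its mesh is clicked.
; If CanBePlanted is set, the click removes the widgets it finds in the world, then creates a Seed_Selection widget and adds it to the viewport.
; It passes a reference to itself to the widget.
; Tick and the construction script are empty, and a PlantTower1 debug print is left unconnected.
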(event `self.ReceiveTick`
  (params (DeltaSeconds :type "Float (single-precision)")))

(event `self.StaticMesh.OnClicked`
  (params (TouchedComponent :type "PrimitiveComponent Object Reference") (ButtonPressed :type "Key Structure"))
  ;[1 1 1] check if can be planted and created widegt
  (if (`self.CanBePlanted`)
    (bind _foundwidgets (`WidgetBlueprintLibrary.GetAllWidgetsOfClass` null false))
    (for _array_element _foundwidgets
      (`Widget.RemoveFromParent` _array_element))
    (bind _returnvalue (`|CreateWidget` "/Game/newTrial/Seed_spawn/Seed_Selection.Seed_Selection_C"))
    (`UserWidget.AddToViewport` _returnvalue 0)
    (set `/Game/newTrial/Seed_spawn/Seed_Selection.Seed_SpawnerBPreference` self _returnvalue)))

(fn `UserConstructionScript`)
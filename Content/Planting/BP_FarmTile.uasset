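; Farm tile where the player plants one of three seedling types, waits for it to grow and harvests it.
; PlantSeed spends the seedling selected on Camera_Pawn, and a macro Delay loop counts down growth in seconds.
; Disease rolls before and after the mesh swap can halt growth and apply a diseased material.
; Activate calls Harvest, which clears the tile and spawns the matching loose-plant actor for healthy crops only.
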(event `self.ReceiveBeginPlay`
  (`Text3DComponent.SetText` (`self.Text3D`) (`self.Value`)))

(event `Plant seedling 3`
  (bind _relativetransformlocation (`self.relativetransformlocation`))
  (bind _returnvalue (`AddComponent|NODE_AddStaticMeshComponent-5` :`RelativeTransform` (`KismetMathLibrary.MakeTransform` _relativetransformlocation)))
  (`self.Grow time` (`self.Seedling3GrowTime`)
    (:`Out`
      (`self.ChanceOfDisease` _returnvalue
        (:`No Disease`
          (`ActorComponent.K2_DestroyComponent` _returnvalue)
          (bind _returnvalue_2 (`AddComponent|NODE_AddStaticMeshComponent-6` :`RelativeTransform` (`KismetMathLibrary.MakeTransform` _relativetransformlocation)))
          (`self.ChanceOfDisease` _returnvalue_2
            (:`No Disease`
              (set `self.FullyGrown?` true)
              (set `self.Curreent Mesh` _returnvalue_2)
              (set `self.WhatCanBeHarvested` "Purpulas Tetra"))))))))

(event `Plant Seedling 2`
  (bind _relativetransformlocation (`self.relativetransformlocation`))
  (bind _returnvalue (`AddComponent|NODE_AddStaticMeshComponent-3` :`RelativeTransform` (`KismetMathLibrary.MakeTransform` _relativetransformlocation)))
  (`self.Grow time` (`self.Seedling2GrowTime`)
    (:`Out`
      (`self.ChanceOfDisease` _returnvalue
        (:`No Disease`
          (`ActorComponent.K2_DestroyComponent` _returnvalue)
          (bind _returnvalue_2 (`AddComponent|NODE_AddStaticMeshComponent-4` :`RelativeTransform` (`KismetMathLibrary.MakeTransform` _relativetransformlocation)))
          (`self.ChanceOfDisease` _returnvalue_2
            (:`No Disease`
              (set `self.FullyGrown?` true)
              (set `self.Curreent Mesh` _returnvalue_2)
              (set `self.WhatCanBeHarvested` "Hydranna Greena"))))))))

(event `Plant Seedling 1`
  (bind _relativetransformlocation (`self.relativetransformlocation`))
  (bind _returnvalue (`AddComponent|NODE_AddStaticMeshComponent-0` :`RelativeTransform` (`KismetMathLibrary.MakeTransform` _relativetransformlocation)))
  (`self.Grow time` (`self.Seedling1GrowTime`)
    (:`Out`
      (`self.ChanceOfDisease` _returnvalue
        (:`No Disease`
          (`ActorComponent.K2_DestroyComponent` _returnvalue)
          (bind _returnvalue_2 (`AddComponent|NODE_AddStaticMeshComponent-2` :`RelativeTransform` (`KismetMathLibrary.MakeTransform` _relativetransformlocation)))
          (`self.ChanceOfDisease` _returnvalue_2
            (:`No Disease`
              (set `self.FullyGrown?` true)
              (set `self.Curreent Mesh` _returnvalue_2)
              (set `self.WhatCanBeHarvested` "Primera Rosa"))))))))

(event `/Game/Planting/BPI_Plant_Seed.Plant Seed`
  (if (not (`self.IsSomethingPlanted`))
    (bind _ascamera_pawn (cast `/Game/TopDownBP/Blueprints/Camera_Pawn` (`GameplayStatics.GetPlayerPawn` 0)))
    (switch `int` (`/Game/TopDownBP/Blueprints/Camera_Pawn.Seed` _ascamera_pawn)
      (:`0`
        (`self.DoWeHaveSeedling1`
          (:`output`
            (`self.Plant Seedling 1`))))
      (:`1`
        (`self.DoWeHaveSeedling2`
          (:`output`
            (`self.Plant Seedling 2`))))
      (:`2`
        (`self.DoWeHaveSeedling3`
          (:`output`
            (`self.Plant seedling 3`)))))
    (set `self.IsSomethingPlanted` true)))

(event `/Game/Planting/BPI_Activate.Activate`
  (`self.Harvest`))

(fn `Harvest`
  (bind _returnvalue (`KismetMathLibrary.Conv_VectorToTransform` (`SceneComponent.K2_GetComponentLocation` (`self.StaticMesh1`))))
  (if (`self.FullyGrown?`)
    (`ActorComponent.K2_DestroyComponent` (`self.Curreent Mesh`))
    (switch `string` (`self.WhatCanBeHarvested`)
      (:`Default`
        _)
      (:`Primera Rosa`
        (`|SpawnActorFromClass` "/Game/Planting/BP_LoosePrimeraRosa.BP_LoosePrimeraRosa_C" _returnvalue "Undefined" "OverrideRootScale" null null))
      (:`Hydranna Greena`
        (`|SpawnActorFromClass` "/Game/Planting/BP_LooseHydrannaGreena.BP_LooseHydrannaGreena_C" _returnvalue "Undefined" "OverrideRootScale" null null))
      (:`Purpulas Tetra`
        (`|SpawnActorFromClass` "/Game/Planting/BP_LoosePurpulasTetra.BP_LoosePurpulasTetra_C" _returnvalue "Undefined" "OverrideRootScale" null null)))
    (set `self.FullyGrown?` false)
    (set `self.Curreent Mesh` null)
    (set `self.IsSomethingPlanted` false)
    (set `self.WhatCanBeHarvested` "")))

(fn `UserConstructionScript`)